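; BP_Player is the player Blueprint that handles mouse-driven interaction with widgets.
; On BeginPlay it shows the mouse cursor and sets the first player controller to Game and UI input mode.
; Left mouse press and release are forwarded to a WidgetInteraction component as pointer key events.
; Leftover nodes for spring arm length, a main menu widget and Fire visibility are unconnected and never run.
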(event `self.ReceiveBeginPlay`
  (bind _returnvalue (`GameplayStatics.GetPlayerController` 0))
  (set `PlayerController.bShowMouseCursor` true _returnvalue)
  (`WidgetBlueprintLibrary.SetInputMode_GameAndUIEx` _returnvalue null))

(event `Key|LeftMouseButton`
  (params (Key :type "Key Structure"))
  (bind _widgetinteraction (`self.WidgetInteraction`))
  (:`Pressed`
    (`WidgetInteractionComponent.PressPointerKey` _widgetinteraction Key))
  (:`Released`
    (`WidgetInteractionComponent.ReleasePointerKey` _widgetinteraction "None")))

(event `Key|RightMouseButton`
  (params (Key :type "Key Structure")))

(fn `UserConstructionScript`)